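; Hand grenade actor that explodes on a timer after BeginPlay and shows a player-facing world-space indicator, scaled by distance within a clamped range.
; Explode fires a radial force impulse, hides the grenade and plays sound, camera shake and heat distortion.
; A line trace to a fixed world point below the origin places particles and a randomized burn decal.
; A sphere overlap flags targets, barrels, gas tanks, walls and characters to explode or ragdoll.
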(event EventBeginPlay
  (bind _radialforce (Variables|Default|GetRadialForce))
  (Utilities|FlowControl|Sequence
    (:then_0
      ;[1 1 1] Set radial force values at start
      (Variables|/Script/Engine.RadialForceComponent|SetForceStrength _radialforce (Variables|ExplosionSettings|GetexplosionForceStrength))
      (Variables|/Script/Engine.RadialForceComponent|SetImpulseStrength _radialforce (Variables|ExplosionSettings|GetexplosionImpulseStrength))
      (Variables|/Script/Engine.RadialForceComponent|SetRadius _radialforce (Variables|ExplosionSettings|GetexplosionRadius)))
    (:then_1
      ;[1 1 1] Explode after set amount of time
      (Utilities|FlowControl|Delay (Variables|ExplosionSettings|GetexplosionTimer))
      (CallFunction|Explode))))

(event EventTick
  (params (DeltaSeconds :type Float%20%28single-precision%29))
  (bind _worldspacewidget (Variables|Default|GetworldSpaceWidget))
  ;[1 1 1] Make grenade indicator always face player
  (Transformation|SetWorldRotation _worldspacewidget (Math|Rotator|FindLookatRotation (Transformation|GetWorldLocation _worldspacewidget) (Transformation|GetActorLocation (Game|Player|GetPlayerPawn 0))) false false)
  ;[1 1 1] Set grenade UI scale based on distance to player
  (Utilities|FlowControl|Sequence
    (:then_0
      (Variables|Default|SetuiRenderScale (Math|Float|Clamp(Float) (* (stale _output_get) 0.0007) 1.25 1.5)) ; Set ui render scale float value
    )
    (:then_1
      (bind _output_get (Variables|Default|SetdistanceToPlayer (Transformation|GetDistanceTo (Game|GetPlayerCharacter 0)))) ; Set distance value
    )
    (:then_2
      (bind _asbp_ui_grenade_world_space (Utilities|Casting|CastToBP_UI_Grenade_WorldSpace (UserInterface|GetUserWidgetObject (Variables|Default|GetworldSpaceWidget)))) ; Cast to widget component
      (Widget|Transform|SetRenderScale _asbp_ui_grenade_world_space (Math|Vector2D|MakeVector2D (Variables|Default|GetuiRenderScale) (Variables|Default|GetuiRenderScale))) ; Set UI render scale
    )))

(fn ConstructionScript)

(fn Explode
  (bind _returnvalue (Math|Random|RandomFloatinRange 1e+02 3e+02))
  (bind _hand_grenade_01 (Variables|Default|GetHand_Grenade_01))
  (bind _hand_grenade_01_2 (Variables|Default|GetHand_Grenade_01))
  (bind _returnvalue_2 (Transformation|GetWorldLocation _hand_grenade_01_2))
  (bind _returnvalue_3 (Transformation|GetWorldLocation _hand_grenade_01))
  (Class|RadialForceComponent|FireImpulse (Variables|Default|GetRadialForce)) ; Fire radial force impulse
  (Utilities|FlowControl|Sequence
    (:then_0
      ;[1 1 1] Spawn Explosion Particles
      (bind (_outhit _returnvalue_4) (Collision|LineTraceByChannel _returnvalue_2 "0, 0,-5000.000000" "TraceTypeQuery1" false 0 "None"))
      (if _returnvalue_4
        (Utilities|FlowControl|Sequence
          (:then_0
            (Effects|SpawnEmitteratLocation "/Game/Low_Poly_FPS_Pack/Content/Particle_Systems/Explosions/PS_Explosion.PS_Explosion" (.Location (Collision|BreakHitResult _outhit)) "0, 0, 0" (Math|Conversions|ToVector(Float) (Math|Random|RandomFloatinRange 0.8 1.2)))
            (Game|SpawnActorfromClass "/Game/Low_Poly_FPS_Pack/Content/Blueprints/Demo_Maps/Effects/BP_Heat_Distortion_Effect.BP_Heat_Distortion_Effect_C" (Math|Transform|MakeTransform _returnvalue_2 "0, 0, 0" "1,1,1") "AlwaysSpawn" 0 0) ; Spawn heat distortion effect
          )
          (:then_1
            (bind _returnvalue_5 (Rendering|Decal|SpawnDecalatLocation "/Game/Low_Poly_FPS_Pack/Content/Materials/Material_Instances/Decals/MI_Decal_Burn_Mark_01.MI_Decal_Burn_Mark_01" (Math|Vector|MakeVector _returnvalue _returnvalue _returnvalue) (.Location (Collision|BreakHitResult _outhit)) (Math|Conversions|RotationFromXVector (.Normal (Collision|BreakHitResult _outhit))) 3e+02))
            (Transformation|SetRelativeRotation _returnvalue_5 (Math|Rotator|MakeRotator (Math|Random|RandomFloatinRange 0.0 3.6e+02) (.Pitch (Math|Rotator|BreakRotator (Math|Conversions|RotationFromXVector (.Normal (Collision|BreakHitResult _outhit))))) (.Yaw (Math|Rotator|BreakRotator (Math|Conversions|RotationFromXVector (.Normal (Collision|BreakHitResult _outhit)))))) false false)))))
    (:then_1
      ;[1 1 1] Hide projectile and play explosion sound effect
      (Rendering|SetVisibility (Variables|Default|GetHand_Grenade_01) false false)
      (Rendering|SetVisibility (Variables|Default|GetworldSpaceWidget) false false)
      (Audio|PlaySoundatLocation "/Game/Low_Poly_FPS_Pack/Content/Audio/Sound_Cues/Explosions/SC_Explosion_Random.SC_Explosion_Random" _returnvalue_3 "0, 0, 0" 1.0 1.0 0.0 "/Game/Low_Poly_FPS_Pack/Content/Audio/Sound_Attenuation/SoundAttenuation_Main.SoundAttenuation_Main")
      (Camera|PlayWorldCameraShake "/Game/Low_Poly_FPS_Pack/Content/Blueprints/Camera_Shake/BP_Camera_Shake_Small.BP_Camera_Shake_Small_C" _returnvalue_3 0.0 2.5e+03 1.0 true) ; Play camera shake effect
    )
    (:then_2
      ;[1 1 1] Sphere overlap check for actors within radius
      (bind (_outactors _returnvalue_6) (Collision|SphereOverlapActors (Transformation|GetWorldLocation (Variables|Default|GetHand_Grenade_01)) (Variables|/Script/Engine.RadialForceComponent|GetRadius (Variables|Default|GetRadialForce)) (Utilities|Array|MakeArray "ObjectTypeQuery4" "ObjectTypeQuery2" "ObjectTypeQuery1") 0))
      (if _returnvalue_6
        (for _array_element _outactors
          (Utilities|FlowControl|Sequence
            (:then_0
              ;[1 1 1] Check which actors got hit by sphere overlap
              (bind _asbp_target (Utilities|Casting|CastToBP_Target _array_element))
              (if (not (Variables|/Game/Low_Poly_FPS_Pack/Content/Blueprints/Demo_Maps/Enivronment_Props/Target/BP_Target.BP_Target_C|GettargetHasExploded _asbp_target))
                (Variables|/Game/Low_Poly_FPS_Pack/Content/Blueprints/Demo_Maps/Enivronment_Props/Target/BP_Target.BP_Target_C|SetexplodeTarget _asbp_target true)))
            (:then_1
              (bind _asbp_explosive_barrel (Utilities|Casting|CastToBP_Explosive_Barrel _array_element))
              (if (not (Variables|/Game/Low_Poly_FPS_Pack/Content/Blueprints/Demo_Maps/Enivronment_Props/Explosive_Barrel/BP_Explosive_Barrel.BP_Explosive_Barrel_C|GetbarrelIsHit _asbp_explosive_barrel))
                (Variables|/Game/Low_Poly_FPS_Pack/Content/Blueprints/Demo_Maps/Enivronment_Props/Explosive_Barrel/BP_Explosive_Barrel.BP_Explosive_Barrel_C|SetbarrelIsHit _asbp_explosive_barrel true)))
            (:then_2
              (bind _asbp_gas_tank (Utilities|Casting|CastToBP_Gas_Tank _array_element))
              (if (not (Variables|/Game/Low_Poly_FPS_Pack/Content/Blueprints/Demo_Maps/Enivronment_Props/Gas_Tank/BP_Gas_Tank.BP_Gas_Tank_C|GetgasTankIsHit _asbp_gas_tank))
                (Variables|/Game/Low_Poly_FPS_Pack/Content/Blueprints/Demo_Maps/Enivronment_Props/Gas_Tank/BP_Gas_Tank.BP_Gas_Tank_C|SetgasTankIsHit _asbp_gas_tank true)))
            (:then_3
              (bind _asbp_stone_wall (Utilities|Casting|CastToBP_Stone_Wall _array_element))
              (if (not (Variables|/Game/Low_Poly_FPS_Pack/Content/Blueprints/Demo_Maps/Enivronment_Props/Stone_Wall/BP_Stone_Wall.BP_Stone_Wall_C|GetwallHasExploded _asbp_stone_wall))
                (Variables|/Game/Low_Poly_FPS_Pack/Content/Blueprints/Demo_Maps/Enivronment_Props/Stone_Wall/BP_Stone_Wall.BP_Stone_Wall_C|SetexplodeWall _asbp_stone_wall true)))
            (:then_4
              (bind _asbp_tpc_weapon_base (Utilities|Casting|CastToBP_TPC_Weapon_Base _array_element)) ; If explosion hits third person character
              (if (not (Variables|/Game/Low_Poly_FPS_Pack/Content/Blueprints/Third_Person_Character/Base/BP_TPC_Weapon_Base.BP_TPC_Weapon_Base_C|GethasRagdolled _asbp_tpc_weapon_base))
                (Variables|/Game/Low_Poly_FPS_Pack/Content/Blueprints/Third_Person_Character/Base/BP_TPC_Weapon_Base.BP_TPC_Weapon_Base_C|SetenableRagdoll _asbp_tpc_weapon_base true)))))))))