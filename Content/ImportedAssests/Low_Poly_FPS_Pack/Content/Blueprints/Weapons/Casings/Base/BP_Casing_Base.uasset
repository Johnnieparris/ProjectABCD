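; Base Blueprint for ejected weapon shell casings that spin, make a landing-style sound and clean themselves up.
; Tick rotates the casing mesh in roll and pitch at a configurable speed scaled by delta time.
; BeginPlay starts two timed branches: one destroys the actor after a set lifetime, the other plays the casing sound at the mesh location after a short random delay.
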(event EventBeginPlay
  ;[1 1 1] Destroy casing after set amount of time
  (Utilities|FlowControl|Sequence
    (:then_0
      (Utilities|FlowControl|Delay (Variables|DestroySettings|GetdestroyTimer)) ; Amount of sec before bullet is destroyed
      (Actor|DestroyActor))
    (:then_1
      ;[1 1 1] Play random casing sound
      (Utilities|FlowControl|Delay (Math|Random|RandomFloatinRange 0.2 0.6))
      (Audio|PlaySoundatLocation (Variables|SoundSettings|GetcasingSound) (Transformation|GetWorldLocation (Variables|Default|Getcasing_mesh))))))

(event EventTick
  (params (DeltaSeconds :type Float%20%28single-precision%29))
  (bind _rotationspeed (Variables|RotationSettings|GetrotationSpeed))
  ;[1 1 1] Casing rotation over time
  (Transformation|AddLocalRotation (Variables|Default|Getcasing_mesh) (Math|Rotator|MakeRotator (* DeltaSeconds _rotationspeed) (* DeltaSeconds _rotationspeed) 0.0) false false))

(fn ConstructionScript)