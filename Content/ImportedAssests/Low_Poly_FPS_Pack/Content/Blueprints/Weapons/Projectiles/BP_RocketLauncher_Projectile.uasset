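; Rocket launcher projectile that faces its velocity, explodes on its first hit, or is destroyed after a timer.
; Explode fires a radial force impulse, spawns effects, burn decal, sound and camera shake, then hides the rocket.
; A sphere overlap casts to specific destructible classes and the third-person character, setting their explode, hit or ragdoll flags.
; When the launcher character's camera follows the projectile, player input is disabled until removal.
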(event EventBeginPlay
  (bind _radialforce (Variables|Default|GetRadialForce))
  (Utilities|FlowControl|Sequence
    (:then_0
      ;[1 1 1] Cast to launcher BP base
      (bind _asbp_launcher_weapon_base (Utilities|Casting|CastToBP_Launcher_Weapon_Base (Game|GetPlayerCharacter 0)))
      (Variables|Default|SetcastedCharacter _asbp_launcher_weapon_base))
    (:then_1
      ;[1 1 1] Set speed and radial force values at start
      (Variables|/Script/Engine.RadialForceComponent|SetForceStrength _radialforce (Variables|ExplosionSettings|GetexplosionForceStrength))
      (Variables|/Script/Engine.RadialForceComponent|SetImpulseStrength _radialforce (Variables|ExplosionSettings|GetexplosionImpulseStrength))
      (Variables|/Script/Engine.RadialForceComponent|SetRadius _radialforce (Variables|ExplosionSettings|GetexplosionRadius))
      (Utilities|FlowControl|Sequence
        (:then_0
          ;[1 1 1] Disable player input while projectile is active (if enabled and valid)
          (Utilities|IsValid (Variables|Default|GetcastedCharacter)
            (:Is%20Valid
              (if (Variables|/Game/Low_Poly_FPS_Pack/Content/Blueprints/Arms/Base/BP_Launcher_Weapon_Base.BP_Launcher_Weapon_Base_C|GetcameraFollowProjectile (Variables|Default|GetcastedCharacter))
                (Input|DisableInput (Variables|Default|GetcastedCharacter) (Game|GetPlayerController 0))))))
        (:then_1
          ;[1 1 1] Destroy projectile after set amount of time
          (Utilities|FlowControl|Delay (Variables|ProjectileSettings|GetdestroyTimer))
          (Utilities|FlowControl|Sequence
            (:then_0
              ;[1 1 1] Enable player input again after projectile has exploded (if enabled and valid)
              (Utilities|IsValid (Variables|Default|GetcastedCharacter)
                (:Is%20Valid
                  (if (Variables|/Game/Low_Poly_FPS_Pack/Content/Blueprints/Arms/Base/BP_Launcher_Weapon_Base.BP_Launcher_Weapon_Base_C|GetcameraFollowProjectile (Variables|Default|GetcastedCharacter))
                    (Input|EnableInput (Variables|Default|GetcastedCharacter) (Game|GetPlayerController 0))))))
            (:then_1
              (Actor|DestroyActor))))))))

(event Collision|EventHit
  (params (MyComp :type Primitive%20Component%20Object%20Reference) (Other :type Actor%20Object%20Reference) (OtherComp :type Primitive%20Component%20Object%20Reference) (bSelfMoved :type Boolean) (HitLocation :type Vector :default "0, 0, 0") (HitNormal :type Vector :default "0, 0, 0") (NormalImpulse :type Vector :default "0, 0, 0") (Hit :type Hit%20Result%20Structure%20%28by%20ref%29))
  (bind _castedcharacter (Variables|Default|GetcastedCharacter))
  (bind _castedcharacter_2 (Variables|Default|GetcastedCharacter))
  ;[1 1 1] Check if projectile actor hits something, and set hit location and hit normal
  (Variables|HitCheck|SethitLocation HitLocation)
  (Variables|HitCheck|SethitNormal HitNormal)
  (if (not (Variables|HitCheck|GethasExploded))
    (CallFunction|Explode) ; If hit something, explode projectile
    (Utilities|IsValid _castedcharacter_2
      (:Is%20Valid
        (if (Variables|/Game/Low_Poly_FPS_Pack/Content/Blueprints/Arms/Base/BP_Launcher_Weapon_Base.BP_Launcher_Weapon_Base_C|GetcameraFollowProjectile _castedcharacter_2)
          (Utilities|FlowControl|Delay 0.1)
          (else
            (Utilities|FlowControl|Delay 2.0)))
        (Utilities|FlowControl|Sequence
          (:then_0
            ;[1 1 1] Enable player input again after projectile has exploded (if enabled and valid)
            (Utilities|IsValid _castedcharacter
              (:Is%20Valid
                (if (Variables|/Game/Low_Poly_FPS_Pack/Content/Blueprints/Arms/Base/BP_Launcher_Weapon_Base.BP_Launcher_Weapon_Base_C|GetcameraFollowProjectile _castedcharacter)
                  (Input|EnableInput _castedcharacter (Game|GetPlayerController 0))))))
          (:then_1
            (Actor|DestroyActor)))))))

(event EventTick
  (params (DeltaSeconds :type Float%20%28single-precision%29))
  (bind _rocket_launcher_projectile (Variables|Default|Getrocket_launcher_projectile))
  ;[1 1 1] Rotate projectile to face velocity direction
  (Transformation|SetRelativeRotation _rocket_launcher_projectile (Math|Conversions|RotationFromXVector (Transformation|GetComponentVelocity _rocket_launcher_projectile)) false false))

(fn ConstructionScript)

(fn Explode
  (bind _returnvalue (Math|Random|RandomFloatinRange 1.5e+02 2.7e+02))
  (bind _rocket_launcher_projectile (Variables|Default|Getrocket_launcher_projectile))
  (bind _p_rocket_smoke (Variables|Default|GetP_Rocket_Smoke))
  (bind _hitnormal (Variables|HitCheck|GethitNormal))
  (bind _hitlocation (Variables|HitCheck|GethitLocation))
  (bind _returnvalue_2 (Transformation|GetWorldLocation _rocket_launcher_projectile))
  (bind _returnvalue_3 (Math|Conversions|RotationFromXVector _hitnormal))
  (bind (_roll _pitch _yaw) (Math|Rotator|BreakRotator _returnvalue_3))
  (Variables|HitCheck|SethasExploded true)
  (Class|RadialForceComponent|FireImpulse (Variables|Default|GetRadialForce)) ; Fire radial force impulse
  (Utilities|FlowControl|Sequence
    (:then_0
      ;[1 1 1] Spawn Explosion Particles
      (Utilities|FlowControl|Sequence
        (:then_0
          (Effects|SpawnEmitteratLocation "/Game/Low_Poly_FPS_Pack/Content/Particle_Systems/Explosions/PS_Explosion_Spherical.PS_Explosion_Spherical" _hitlocation "0, 0, 0" (Math|Conversions|ToVector(Float) (Math|Random|RandomFloatinRange 1.0 1.7)))
          (Game|SpawnActorfromClass "/Game/Low_Poly_FPS_Pack/Content/Blueprints/Demo_Maps/Effects/BP_Heat_Distortion_Effect.BP_Heat_Distortion_Effect_C" (Math|Transform|MakeTransform _hitlocation "0, 0, 0" "1,1,1") "AlwaysSpawn" 0 0) ; Spawn heat distortion effect
        )
        (:then_1
          (bind _returnvalue_4 (Rendering|Decal|SpawnDecalatLocation "/Game/Low_Poly_FPS_Pack/Content/Materials/Material_Instances/Decals/MI_Decal_Burn_Mark_01.MI_Decal_Burn_Mark_01" (Math|Vector|MakeVector _returnvalue _returnvalue _returnvalue) _hitlocation _returnvalue_3 3e+02))
          (Transformation|SetRelativeRotation _returnvalue_4 (Math|Rotator|MakeRotator (Math|Random|RandomFloatinRange 0.0 3.6e+02) _pitch _yaw) false false))))
    (:then_1
      ;[1 1 1] Hide projectile and play explosion sound effect
      (Rendering|SetVisibility _rocket_launcher_projectile false false)
      (Physics|SetSimulatePhysics _rocket_launcher_projectile false)
      (Audio|PlaySoundatLocation "/Game/Low_Poly_FPS_Pack/Content/Audio/Sound_Cues/Explosions/SC_Explosion_Random.SC_Explosion_Random" _returnvalue_2 "0, 0, 0" 1.0 1.0 0.0 "/Game/Low_Poly_FPS_Pack/Content/Audio/Sound_Attenuation/SoundAttenuation_Main.SoundAttenuation_Main")
      (Camera|PlayWorldCameraShake "/Game/Low_Poly_FPS_Pack/Content/Blueprints/Camera_Shake/BP_Camera_Shake_Big.BP_Camera_Shake_Big_C" _returnvalue_2 0.0 5e+03 1.0 true) ; Play camera shake effect
      ;[1 1 1] Detach smoke particles from projectile
      (Transformation|DetachFromComponent _p_rocket_smoke "KeepWorld" "KeepWorld" "KeepWorld" true)
      (Components|Activation|SetActive _p_rocket_smoke false false))
    (:then_2
      ;[1 1 1] Sphere overlap check for actors within radius
      (bind (_outactors _returnvalue_5) (Collision|SphereOverlapActors (Transformation|GetWorldLocation (Variables|Default|Getrocket_launcher_projectile)) (Variables|/Script/Engine.RadialForceComponent|GetRadius (Variables|Default|GetRadialForce)) (Utilities|Array|MakeArray "ObjectTypeQuery4" "ObjectTypeQuery2" "ObjectTypeQuery1") 0))
      (if _returnvalue_5
        (for _array_element _outactors
          (Utilities|FlowControl|Sequence
            (:then_0
              ;[1 1 1] Check which actors got hit by sphere overlap
              (bind _asbp_target (Utilities|Casting|CastToBP_Target _array_element))
              (if (not (Variables|/Game/Low_Poly_FPS_Pack/Content/Blueprints/Demo_Maps/Enivronment_Props/Target/BP_Target.BP_Target_C|GettargetHasExploded _asbp_target))
                (Variables|/Game/Low_Poly_FPS_Pack/Content/Blueprints/Demo_Maps/Enivronment_Props/Target/BP_Target.BP_Target_C|SetexplodeTarget _asbp_target true)))
            (:then_1
              (bind _asbp_explosive_barrel (Utilities|Casting|CastToBP_Explosive_Barrel _array_element))
              (if (not (Variables|/Game/Low_Poly_FPS_Pack/Content/Blueprints/Demo_Maps/Enivronment_Props/Explosive_Barrel/BP_Explosive_Barrel.BP_Explosive_Barrel_C|GetbarrelIsHit _asbp_explosive_barrel))
                (Variables|/Game/Low_Poly_FPS_Pack/Content/Blueprints/Demo_Maps/Enivronment_Props/Explosive_Barrel/BP_Explosive_Barrel.BP_Explosive_Barrel_C|SetbarrelIsHit _asbp_explosive_barrel true)))
            (:then_2
              (bind _asbp_gas_tank (Utilities|Casting|CastToBP_Gas_Tank _array_element))
              (if (not (Variables|/Game/Low_Poly_FPS_Pack/Content/Blueprints/Demo_Maps/Enivronment_Props/Gas_Tank/BP_Gas_Tank.BP_Gas_Tank_C|GetgasTankIsHit _asbp_gas_tank))
                (Variables|/Game/Low_Poly_FPS_Pack/Content/Blueprints/Demo_Maps/Enivronment_Props/Gas_Tank/BP_Gas_Tank.BP_Gas_Tank_C|SetgasTankIsHit _asbp_gas_tank true)))
            (:then_3
              (bind _asbp_stone_wall (Utilities|Casting|CastToBP_Stone_Wall _array_element))
              (if (not (Variables|/Game/Low_Poly_FPS_Pack/Content/Blueprints/Demo_Maps/Enivronment_Props/Stone_Wall/BP_Stone_Wall.BP_Stone_Wall_C|GetwallHasExploded _asbp_stone_wall))
                (Variables|/Game/Low_Poly_FPS_Pack/Content/Blueprints/Demo_Maps/Enivronment_Props/Stone_Wall/BP_Stone_Wall.BP_Stone_Wall_C|SetexplodeWall _asbp_stone_wall true)))
            (:then_4
              (bind _asbp_house_explosion_area (Utilities|Casting|CastToBP_House_Explosion_Area _array_element))
              (if (not (Variables|/Game/Low_Poly_FPS_Pack/Content/Blueprints/Demo_Maps/Enivronment_Props/Houses/Explosion_Area/BP_House_Explosion_Area.BP_House_Explosion_Area_C|GethouseHasExploded _asbp_house_explosion_area))
                (Variables|/Game/Low_Poly_FPS_Pack/Content/Blueprints/Demo_Maps/Enivronment_Props/Houses/Explosion_Area/BP_House_Explosion_Area.BP_House_Explosion_Area_C|SetexplodeHouse _asbp_house_explosion_area true)))
            (:then_5
              (bind _asbp_watchtower (Utilities|Casting|CastToBP_Watchtower _array_element))
              (if (not (Variables|/Game/Low_Poly_FPS_Pack/Content/Blueprints/Demo_Maps/Enivronment_Props/Watchtower/BP_Watchtower.BP_Watchtower_C|GethasExploded _asbp_watchtower))
                (Variables|/Game/Low_Poly_FPS_Pack/Content/Blueprints/Demo_Maps/Enivronment_Props/Watchtower/BP_Watchtower.BP_Watchtower_C|Setexplode _asbp_watchtower true)))
            (:then_6
              (bind _asbp_tpc_weapon_base (Utilities|Casting|CastToBP_TPC_Weapon_Base _array_element)) ; If explosion hits third person character
              (if (not (Variables|/Game/Low_Poly_FPS_Pack/Content/Blueprints/Third_Person_Character/Base/BP_TPC_Weapon_Base.BP_TPC_Weapon_Base_C|GethasRagdolled _asbp_tpc_weapon_base))
                (Variables|/Game/Low_Poly_FPS_Pack/Content/Blueprints/Third_Person_Character/Base/BP_TPC_Weapon_Base.BP_TPC_Weapon_Base_C|SetenableRagdoll _asbp_tpc_weapon_base true)))))))))