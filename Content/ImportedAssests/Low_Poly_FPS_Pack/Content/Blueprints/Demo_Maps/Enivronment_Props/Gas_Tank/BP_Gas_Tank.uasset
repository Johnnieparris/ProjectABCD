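; Explosive gas tank prop that, once hit, flames and moves on physics thrusters, then explodes after a timer and destroys itself.
; Tick polls a hit flag to start the sequence; radial force values are randomized at BeginPlay.
; Explode spawns effects, sound, a traced scorch decal and a wreck actor, then fires a radial impulse.
; A sphere overlap sets flags on nearby destructibles, tanks and characters, enabling chain reactions and ragdolls.
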(event EventBeginPlay
  (bind _radialforce (Variables|Default|GetRadialForce))
  ;[1 1 1] Set radial force values at start
  (Utilities|FlowControl|Sequence
    (:then_0
      (Variables|/Script/Engine.RadialForceComponent|SetRadius _radialforce (Math|Random|RandomFloatinRange (Variables|ExplosionSettings|GetminExplosionRadius) (Variables|ExplosionSettings|GetmaxExplosionRadius))))
    (:then_1
      (Variables|/Script/Engine.RadialForceComponent|SetForceStrength _radialforce (Math|Random|RandomFloatinRange (Variables|ExplosionSettings|GetminForceStrength) (Variables|ExplosionSettings|GetmaxForceStrength))))
    (:then_2
      (Variables|/Script/Engine.RadialForceComponent|SetImpulseStrength _radialforce (Math|Random|RandomFloatinRange (Variables|ExplosionSettings|GetminImpulseStrength) (Variables|ExplosionSettings|GetmaxImpulseStrength))))))

(event EventTick
  (params (DeltaSeconds :type Float%20%28single-precision%29))
  (bind _flame_audio (Variables|Default|GetFlame_Audio))
  (bind _p_gas_tank_flames (Variables|Default|GetP_Gas_Tank_Flames))
  (if (and (Variables|Default|GetgasTankIsHit) (Variables|Default|GetisInactive)) ; Check every frame if gas tank has been hit
    (Variables|Default|SetgasTankIsHit false)
    (Variables|Default|SetisInactive false)
    (Components|Activation|ToggleActive (Variables|Default|GetPhysicsThruster)) ; Enable physics thrusters
    (Utilities|FlowControl|Sequence
      (:then_0
        ;[1 1 1] Activate/deactivate flame particle system
        (Components|Activation|Activate _p_gas_tank_flames false)
        ;[1 1 1] Activate/deactivate gas tank audio
        (Components|Activation|Activate _flame_audio false))
      (:then_1
        (Utilities|FlowControl|Delay (Variables|ExplosionSettings|GetexplodeTimer)) ; Wait for set amount of time before exploding
        (CallFunction|Explode)
        (Components|Activation|Deactivate _p_gas_tank_flames) ; Deactivate particle system on explode
        (Components|Activation|Deactivate _flame_audio) ; Deactivate sound effect on explode
        (Utilities|FlowControl|Delay 1.5)
        (Actor|DestroyActor) ; Destroy gas tank
      ))))

(fn ConstructionScript)

(fn Explode
  (bind _returnvalue (Math|Random|RandomFloatinRange 1e+02 3e+02))
  (bind _radialforce (Variables|Default|GetRadialForce))
  (bind _gas_tank (Variables|Default|Getgas_tank))
  (bind _gas_tank_2 (Variables|Default|Getgas_tank))
  (bind _returnvalue_2 (Transformation|GetWorldLocation _gas_tank))
  (bind (_x _y _z) (Math|Vector|BreakVector _returnvalue_2))
  (Utilities|FlowControl|Sequence
    (:then_0
      ;[1 1 1] Spawn Explosion Particles
      (Effects|SpawnEmitteratLocation "/Game/Low_Poly_FPS_Pack/Content/Particle_Systems/Explosions/PS_Explosion_Spherical.PS_Explosion_Spherical" _returnvalue_2 "0, 0, 0" (Math|Conversions|ToVector(Float) (Math|Random|RandomFloatinRange 0.8 1.2))) ; Spawn spherical explosion emitter at gas \ntank world location
      (Game|SpawnActorfromClass "/Game/Low_Poly_FPS_Pack/Content/Blueprints/Demo_Maps/Effects/BP_Heat_Distortion_Effect.BP_Heat_Distortion_Effect_C" (Math|Transform|MakeTransform _returnvalue_2 "0, 0, 0" "1,1,1") "AlwaysSpawn" 0 0) ; Spawn heat distortion effect
    )
    (:then_1
      (bind (_outhit _returnvalue_3) (Collision|LineTraceByChannel _returnvalue_2 (Math|Vector|MakeVector _x _y (- _z 5e+01)) "TraceTypeQuery1" false 0 "None"))
      (if _returnvalue_3
        (bind _returnvalue_4 (Rendering|Decal|SpawnDecalatLocation "/Game/Low_Poly_FPS_Pack/Content/Materials/Base_Materials/M_Decal_Base.M_Decal_Base" (Math|Vector|MakeVector _returnvalue _returnvalue _returnvalue) (.Location (Collision|BreakHitResult _outhit)) (Math|Conversions|RotationFromXVector (.Normal (Collision|BreakHitResult _outhit))) (Variables|Default|GetdecalDestroyTimer)))
        (Transformation|SetRelativeRotation _returnvalue_4 (Math|Rotator|MakeRotator (Math|Random|RandomFloatinRange 0.0 3.6e+02) (.Pitch (Math|Rotator|BreakRotator (Math|Conversions|RotationFromXVector (.Normal (Collision|BreakHitResult _outhit))))) (.Yaw (Math|Rotator|BreakRotator (Math|Conversions|RotationFromXVector (.Normal (Collision|BreakHitResult _outhit)))))) false false)))
    (:then_2
      (Game|SpawnActorfromClass "/Game/Low_Poly_FPS_Pack/Content/Blueprints/Demo_Maps/Enivronment_Props/Gas_Tank/Destroyed/BP_Destroyed_Gas_Tank.BP_Destroyed_Gas_Tank_C" (Transformation|GetWorldTransform _radialforce) "AlwaysSpawn" 0 0) ; Spawn destroyed gas tank
      (Class|RadialForceComponent|FireImpulse _radialforce)
      (Components|Activation|SetActive (Variables|Default|GetPhysicsThruster) false false) ; Activate physics thrusters
      ;[1 1 1] Hide gas tank actor and disable collision
      (Rendering|SetVisibility _gas_tank_2 false false)
      (Physics|SetSimulatePhysics _gas_tank_2 false)
      (Collision|SetCollisionEnabled _gas_tank_2 "NoCollision"))
    (:then_3
      (bind (_outactors _returnvalue_5) (Collision|SphereOverlapActors (Transformation|GetWorldLocation _radialforce) (Math|Random|RandomFloatinRange (Variables|ExplosionSettings|GetminExplosionRadius) (Variables|ExplosionSettings|GetmaxExplosionRadius)) (Utilities|Array|MakeArray "ObjectTypeQuery4" "ObjectTypeQuery2" "ObjectTypeQuery1") 0)) ; Check actors within random sphere radius
      (if _returnvalue_5
        (for _array_element _outactors ; Check all actors hit by sphere overlap
          (Utilities|FlowControl|Sequence
            (:then_0
              ;[1 1 1] Check which actors got hit by sphere overlap
              (bind _asbp_target (Utilities|Casting|CastToBP_Target _array_element)) ; If explosion hits target
              (if (not (Variables|/Game/Low_Poly_FPS_Pack/Content/Blueprints/Demo_Maps/Enivronment_Props/Target/BP_Target.BP_Target_C|GettargetHasExploded _asbp_target))
                (Variables|/Game/Low_Poly_FPS_Pack/Content/Blueprints/Demo_Maps/Enivronment_Props/Target/BP_Target.BP_Target_C|SetexplodeTarget _asbp_target true)))
            (:then_1
              (bind _asbp_explosive_barrel (Utilities|Casting|CastToBP_Explosive_Barrel _array_element)) ; If explosion hits other explosive barrels
              (if (not (Variables|/Game/Low_Poly_FPS_Pack/Content/Blueprints/Demo_Maps/Enivronment_Props/Explosive_Barrel/BP_Explosive_Barrel.BP_Explosive_Barrel_C|GetbarrelIsHit _asbp_explosive_barrel))
                (Variables|/Game/Low_Poly_FPS_Pack/Content/Blueprints/Demo_Maps/Enivronment_Props/Explosive_Barrel/BP_Explosive_Barrel.BP_Explosive_Barrel_C|SetbarrelIsHit _asbp_explosive_barrel true)))
            (:then_2
              (bind _asbp_gas_tank (Utilities|Casting|CastToBP_Gas_Tank _array_element)) ; If explosion hits other gas tanks
              (if (not (Variables|BP_Gas_Tank_C|GetgasTankIsHit _asbp_gas_tank))
                (Variables|BP_Gas_Tank_C|SetgasTankIsHit _asbp_gas_tank true)))
            (:then_3
              (bind _asbp_stone_wall (Utilities|Casting|CastToBP_Stone_Wall _array_element)) ; If explosion hits stone wall
              (if (not (Variables|/Game/Low_Poly_FPS_Pack/Content/Blueprints/Demo_Maps/Enivronment_Props/Stone_Wall/BP_Stone_Wall.BP_Stone_Wall_C|GetwallHasExploded _asbp_stone_wall))
                (Variables|/Game/Low_Poly_FPS_Pack/Content/Blueprints/Demo_Maps/Enivronment_Props/Stone_Wall/BP_Stone_Wall.BP_Stone_Wall_C|SetexplodeWall _asbp_stone_wall true)))
            (:then_4
              (bind _asbp_house_explosion_area (Utilities|Casting|CastToBP_House_Explosion_Area _array_element)) ; If explosion hits any house
              (if (not (Variables|/Game/Low_Poly_FPS_Pack/Content/Blueprints/Demo_Maps/Enivronment_Props/Houses/Explosion_Area/BP_House_Explosion_Area.BP_House_Explosion_Area_C|GethouseHasExploded _asbp_house_explosion_area))
                (Variables|/Game/Low_Poly_FPS_Pack/Content/Blueprints/Demo_Maps/Enivronment_Props/Houses/Explosion_Area/BP_House_Explosion_Area.BP_House_Explosion_Area_C|SetexplodeHouse _asbp_house_explosion_area true)))
            (:then_5
              (bind _asbp_watchtower (Utilities|Casting|CastToBP_Watchtower _array_element)) ; If explosion hits watchtower
              (if (not (Variables|/Game/Low_Poly_FPS_Pack/Content/Blueprints/Demo_Maps/Enivronment_Props/Watchtower/BP_Watchtower.BP_Watchtower_C|GethasExploded _asbp_watchtower))
                (Variables|/Game/Low_Poly_FPS_Pack/Content/Blueprints/Demo_Maps/Enivronment_Props/Watchtower/BP_Watchtower.BP_Watchtower_C|Setexplode _asbp_watchtower true)))
            (:then_6
              (bind _asbp_tpc_weapon_base (Utilities|Casting|CastToBP_TPC_Weapon_Base _array_element)) ; If explosion hits third person character
              (if (not (Variables|/Game/Low_Poly_FPS_Pack/Content/Blueprints/Third_Person_Character/Base/BP_TPC_Weapon_Base.BP_TPC_Weapon_Base_C|GethasRagdolled _asbp_tpc_weapon_base))
                (Variables|/Game/Low_Poly_FPS_Pack/Content/Blueprints/Third_Person_Character/Base/BP_TPC_Weapon_Base.BP_TPC_Weapon_Base_C|SetenableRagdoll _asbp_tpc_weapon_base true)))))))
    (:then_4
      ;[1 1 1] Play explosion sound effect
      (Audio|PlaySoundatLocation "/Game/Low_Poly_FPS_Pack/Content/Audio/Sound_Cues/Explosions/SC_Explosion_Random.SC_Explosion_Random" (Transformation|GetWorldLocation (Variables|Default|Getgas_tank)) "0, 0, 0" 1.0 1.0 0.0 "/Game/Low_Poly_FPS_Pack/Content/Audio/Sound_Attenuation/SoundAttenuation_Main.SoundAttenuation_Main" 0 0))))