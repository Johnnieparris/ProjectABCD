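; BP_Stone_Wall is an environment prop for an intact stone wall that can be blown apart.
; Tick polls the ExplodeWall flag, with WallHasExploded guarding against a repeat trigger; nothing in this graph sets ExplodeWall to true.
; When triggered, it spawns BP_Stone_Wall_Destroyed at the wall mesh's world transform, then destroys itself, swapping the intact actor for the destroyed one.
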(event EventTick
  (params (DeltaSeconds :type Float%20%28single-precision%29))
  (bind _sm_stone_wall (Variables|Default|GetSM_stone_wall))
  (if (and (Variables|Default|GetexplodeWall) (not (Variables|Default|GetwallHasExploded)))
    (Variables|Default|SetexplodeWall false)
    (Variables|Default|SetwallHasExploded true)
    (Game|SpawnActorfromClass "/Game/Low_Poly_FPS_Pack/Content/Blueprints/Demo_Maps/Enivronment_Props/Stone_Wall/Destroyed/BP_Stone_Wall_Destroyed.BP_Stone_Wall_Destroyed_C" (Math|Transform|MakeTransform (Transformation|GetWorldLocation _sm_stone_wall) (Transformation|GetWorldRotation _sm_stone_wall) (Transformation|GetWorldScale _sm_stone_wall)) "AdjustIfPossibleButAlwaysSpawn" 0 0) ; Spawn destroyed stone wall
    (Actor|DestroyActor) ; Destroy stone wall actor
  ))

(fn ConstructionScript)