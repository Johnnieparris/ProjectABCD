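; BP_Watchtower_Destroyed is the debris actor for a destroyed watchtower, built from broken chunk and plank meshes.
; BeginPlay starts two timers: one enables settling checks, the other destroys the whole actor.
; Once enabled, Tick turns off physics and collision on each piece with zero velocity.
; A 15-second Delay, started by the first resting piece, then sets a flag that stops the checks.
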(event EventBeginPlay
  (Utilities|FlowControl|Sequence
    (:then_0
      (Utilities|FlowControl|Delay (Variables|Default|GetdisablePhysicsTimer)) ; Disable physics after set amount of time
      (Variables|Default|SetdisablePhysics true))
    (:then_1
      (Utilities|FlowControl|Delay (Variables|Default|GetdestroyTimer)) ; Destroy actor after set amount of time
      (Actor|DestroyActor))))

(event EventTick
  (params (DeltaSeconds :type Float%20%28single-precision%29))
  (if (and (Variables|Default|GetdisablePhysics) (not (Variables|Default|GethasDisabledPhysics))) ; Check if physics has been disabled
    (for _array_element (Utilities|Array|MakeArray (Variables|Default|GetSM_watchtower_destroyed_001) (Variables|Default|GetSM_watchtower_destroyed_002) (Variables|Default|GetSM_watchtower_destroyed_003) (Variables|Default|GetSM_watchtower_destroyed_004) (Variables|Default|GetSM_watchtower_destroyed_005) (Variables|Default|GetSM_watchtower_destroyed_006) (Variables|Default|GetSM_watchtower_destroyed_007) (Variables|Default|GetSM_watchtower_destroyed_008) (Variables|Default|GetSM_watchtower_destroyed_009) (Variables|Default|GetSM_watchtower_destroyed_010) (Variables|Default|GetSM_watchtower_destroyed_011) (Variables|Default|GetSM_watchtower_destroyed_012) (Variables|Default|GetSM_watchtower_destroyed_013) (Variables|Default|GetSM_watchtower_destroyed_014) (Variables|Default|GetSM_watchtower_destroyed_plank_001) (Variables|Default|GetSM_watchtower_destroyed_plank_002) (Variables|Default|GetSM_watchtower_destroyed_plank_003) (Variables|Default|GetSM_watchtower_destroyed_plank_004) (Variables|Default|GetSM_watchtower_destroyed_plank_005) (Variables|Default|GetSM_watchtower_destroyed_plank_006) (Variables|Default|GetSM_watchtower_destroyed_plank_007) (Variables|Default|GetSM_watchtower_destroyed_plank_008) (Variables|Default|GetSM_watchtower_destroyed_plank_009) (Variables|Default|GetSM_watchtower_destroyed_plank_010) (Variables|Default|GetSM_watchtower_destroyed_plank_011) (Variables|Default|GetSM_watchtower_destroyed_plank_012) (Variables|Default|GetSM_watchtower_destroyed_plank_013) (Variables|Default|GetSM_watchtower_destroyed_plank_014) (Variables|Default|GetSM_watchtower_destroyed_plank_015) (Variables|Default|GetSM_watchtower_destroyed_plank_016) (Variables|Default|GetSM_watchtower_destroyed_plank_017)) ; Loop through all destroyed objects
      (if (== (Math|Vector|VectorLength (Transformation|GetComponentVelocity _array_element)) 0.0) ; Check velocity
        (Physics|SetSimulatePhysics _array_element false) ; Disable physics after set amount of time
        (Collision|SetCollisionEnabled _array_element "NoCollision") ; Disable collision after set amount of time
        (Utilities|FlowControl|Delay 15.0)
        (Variables|Default|SethasDisabledPhysics true) ; Stop checking if physics has been disabled
      ))))

(fn ConstructionScript)