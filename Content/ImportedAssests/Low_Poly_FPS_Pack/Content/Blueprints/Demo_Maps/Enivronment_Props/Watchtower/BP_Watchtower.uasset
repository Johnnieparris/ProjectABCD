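; BP_Watchtower is a destructible watchtower environment prop that swaps itself for a destroyed version when triggered.
; Tick polls an Explode flag and, guarded by HasExploded, calls ExplodeWatchtower only once.
; That function spawns BP_Watchtower_Destroyed at the tower mesh's world transform, fires two radial force impulses, then destroys the original actor.
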(event EventBeginPlay)

(event Collision|EventActorBeginOverlap
  (params (OtherActor :type Actor%20Object%20Reference)))

(event EventTick
  (params (DeltaSeconds :type Float%20%28single-precision%29))
  (if (and (Variables|Default|Getexplode) (not (Variables|Default|GethasExploded)))
    (Variables|Default|Setexplode false)
    (Variables|Default|SethasExploded true)
    (CallFunction|ExplodeWatchtower)))

(fn ConstructionScript)

(fn ExplodeWatchtower
  (bind _sm_watchtower (Variables|Default|GetSM_Watchtower))
  (Game|SpawnActorfromClass "/Game/Low_Poly_FPS_Pack/Content/Blueprints/Demo_Maps/Enivronment_Props/Watchtower/Destroyed/BP_Watchtower_Destroyed.BP_Watchtower_Destroyed_C" (Math|Transform|MakeTransform (Transformation|GetWorldLocation _sm_watchtower) (Transformation|GetWorldRotation _sm_watchtower) (Transformation|GetWorldScale _sm_watchtower)) "AdjustIfPossibleButAlwaysSpawn" 0 0) ; Spawn destroyed watchtower
  (Class|RadialForceComponent|FireImpulse (Variables|Default|GetRadialForce))
  (Actor|DestroyActor))