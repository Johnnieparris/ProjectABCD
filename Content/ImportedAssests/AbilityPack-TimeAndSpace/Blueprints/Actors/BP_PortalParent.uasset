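; Parent Blueprint for linked portals that show a live view through OtherPortal and teleport overlapping Characters to it.
; Each Tick moves the other portal's scene capture to mirror the player camera, with a 180-degree yaw flip.
; Mesh overlap moves the Character and sets player 0's control rotation, gated by a short cooldown and trigger volumes that block back entry.
; The construction script assigns the capture's render target and the mesh's portal material.
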(event OnComponentBeginOverlap(Mesh)
  (params (OverlappedComponent :type Primitive%20Component%20Object%20Reference) (OtherActor :type Actor%20Object%20Reference) (OtherComp :type Primitive%20Component%20Object%20Reference) (OtherBodyIndex :type Integer) (bFromSweep :type Boolean) (SweepResult :type Hit%20Result%20Structure%20%28by%20ref%29))
  (bind _otherportal (Variables|Default|GetOtherPortal))
  (bind _teleportlocation (Variables|BP_PortalParent_C|GetTeleportLocation _otherportal))
  (bind _returnvalue (Transformation|GetWorldRotation _teleportlocation))
  ;[0 0 0 0.5 16] Set Your Player Reference Here
  (bind _ascharacter (Utilities|Casting|CastToCharacter OtherActor))
  (Variables|Default|SetPlayer _ascharacter)
  ;[0 0 0 0.5] Teleport to Location and set rotation
  (if (Variables|Default|GetCanTeleport)
    (Variables|Default|SetCanTeleport false)
    (Transformation|SetActorLocationAndRotation (Variables|Default|GetPlayer) (Transformation|GetWorldLocation _teleportlocation) _returnvalue false true)
    (Pawn|SetControlRotation (Game|GetPlayerController 0) _returnvalue)
    (Utilities|FlowControl|Delay 0.5)
    (Variables|Default|SetCanTeleport true)))

(event OnComponentBeginOverlap(TriggerCanTeleport)
  (params (OverlappedComponent :type Primitive%20Component%20Object%20Reference) (OtherActor :type Actor%20Object%20Reference) (OtherComp :type Primitive%20Component%20Object%20Reference) (OtherBodyIndex :type Integer) (bFromSweep :type Boolean) (SweepResult :type Hit%20Result%20Structure%20%28by%20ref%29))
  ;[0 0 0 0.5] Prevent entering from back
  (Variables|Default|SetCanTeleport true))

(event OnComponentBeginOverlap(TriggerCannotTeleport)
  (params (OverlappedComponent :type Primitive%20Component%20Object%20Reference) (OtherActor :type Actor%20Object%20Reference) (OtherComp :type Primitive%20Component%20Object%20Reference) (OtherBodyIndex :type Integer) (bFromSweep :type Boolean) (SweepResult :type Hit%20Result%20Structure%20%28by%20ref%29))
  ;[0 0 0 0.5] Prevent entering from back
  (Variables|Default|SetCanTeleport false))

(event EventBeginPlay
  ;[0 0 0 0.5 16] Set Your Player Reference Here
  (Utilities|FlowControl|Delay 0.2)
  (Actor|SetOwner (Game|GetPlayerCharacter 0)))

(event EventTick
  (params (DeltaSeconds :type Float%20%28single-precision%29))
  (bind _returnvalue (Game|GetPlayerCameraManager 0))
  (bind _otherportal (Variables|Default|GetOtherPortal))
  (bind _defaultsceneroot (Variables|Default|GetDefaultSceneRoot))
  (bind _returnvalue_2 (Transformation|GetWorldTransform _defaultsceneroot))
  (bind _transformcomponent (Variables|/Script/Engine.PlayerCameraManager|GetTransformComponent _returnvalue))
  (bind _defaultsceneroot_2 (Variables|BP_PortalParent_C|GetDefaultSceneRoot _otherportal))
  (bind _returnvalue_3 (Transformation|GetWorldTransform _transformcomponent))
  (bind _returnvalue_4 (Transformation|GetWorldTransform _defaultsceneroot_2))
  (bind (_roll _pitch _yaw) (Math|Rotator|BreakRotator (.rotation _returnvalue_4)))
  (bind _returnvalue_5 (- _yaw 1.8e+02))
  (bind _returnvalue_6 (Math|Rotator|MakeRotator _roll _pitch _returnvalue_5))
  (bind _returnvalue_7 (Math|Rotator|Delta(Rotator) _returnvalue_6 (.rotation _returnvalue_2)))
  ;[0 0 0 0.5] Rotate View
  (Transformation|SetWorldLocationAndRotation (Variables|BP_PortalParent_C|GetPortalSceneCapture (Variables|Default|GetOtherPortal)) (+ (- (.location _returnvalue_4) (Math|Vector|RotateVector (.location _returnvalue_2) _returnvalue_7)) (Math|Vector|RotateVector (.location _returnvalue_3) _returnvalue_7)) (Math|Rotator|CombineRotators (.rotation _returnvalue_3) _returnvalue_7) false false))

(fn ConstructionScript
  ;[0 0 0 0.5] Set Texture
  (Utilities|IsValid (Variables|Default|GetTextureTarget)
    (:Is%20Valid
      (Variables|/Script/Engine.SceneCaptureComponent2D|SetTextureTarget (Variables|Default|GetPortalSceneCapture) (Variables|Default|GetTextureTarget)))
    (:Is%20Not%20Valid
      _))
  (Rendering|Material|SetMaterial (Variables|Default|GetMesh) 0 (Variables|Default|GetPortalMaterial)))