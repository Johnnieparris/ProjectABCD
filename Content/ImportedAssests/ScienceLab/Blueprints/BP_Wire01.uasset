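; Construction-script Blueprint that builds a configurable wire from spline mesh components along a spline.
; SplineMeshVar selects one segment per pair of spline points or segments at fixed Spacing along the length, with tangents scaled by TangentScale.
; WireVar picks among six spline mesh variants, the last three using two material slots, and WireSize scales each segment.
; Dynamic MI_Wire instances receive the colour, dirt, specular, roughness and TextureVar-selected texture settings.
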(fn ConstructionScript
  (|Wire))