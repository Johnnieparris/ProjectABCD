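; Elven bow weapon that charges, reloads and fires BP_Arrow projectiles for the player.
; A timeline drives ChargeAmount, playing on charge start and reversing on charge end, with a separate event to stop and reset it.
; Reload spawns an arrow attached to the bow's ArrowSocket.
; Fire replaces that arrow with a new one spawned at the first-person camera, launches it with ChargeAmount, then clears the reference.
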(event Custom|BeginCharge
  (Variables|Default|GetArrow
    (:then
      (bind _chargeamount (Timeline|ChargeTimeline Play)
        (:Update
          (Variables|Default|SetChargeAmount _chargeamount))))
    (:else)))

(event Custom|ReloadBow
  (bind _returnvalue (Game|SpawnActorfromClass "/Game/weapons/Bow/Arrow/BP_Arrow.BP_Arrow_C" (Math|Transform|MakeTransform "0, 0, 0" "0.000000,90.000000,0.000000" "4.000000,4.000000,4.000000") "AlwaysSpawn" 0 "NewEnumerator3" 0))
  (bind _output_get (Variables|Default|SetArrow _returnvalue))
  (Transformation|AttachComponentToComponent _output_get (Variables|Default|GetElvenBow) "ArrowSocket" "KeepRelative" "KeepRelative" "KeepWorld" true))

(event Custom|EndCharge
  (Variables|Default|GetArrow
    (:then
      (bind _chargeamount (Timeline|ChargeTimeline Reverse)
        (:Update
          (Variables|Default|SetChargeAmount _chargeamount))))
    (:else)))

(event Custom|Fire
  (Variables|Default|GetArrow
    (:then
      (Actor|DestroyActor (Variables|Default|GetArrow))
      (bind _returnvalue (Game|SpawnActorfromClass "/Game/weapons/Bow/Arrow/BP_Arrow.BP_Arrow_C" (Math|Transform|MakeTransform (.location (Transformation|GetWorldTransform (Variables|/Game/ThirdPersonBP/Blueprints/Player.Player_C|GetFirstPersonCamera (.AsPlayer (Utilities|Casting|CastToPlayer (Game|GetPlayerCharacter 0)))))) (Math|Rotator|MakeRotator 0.0 0.0 0.0) "6.000000,6.000000,6.000000") "AlwaysSpawn" 0 "NewEnumerator3" 0))
      (Transformation|DetachFromActor _returnvalue "KeepWorld" "KeepWorld" "KeepWorld")
      (bind _output_get (Variables|Default|SetArrow _returnvalue))
      (Transformation|SetActorRotation (Variables|Default|GetArrow))
      (Default|Fire _output_get (Variables|Default|GetChargeAmount))
      (Variables|Default|SetArrow 0))
    (:else)))

(event Custom|StopCharge
  (Utilities|FlowControl|Sequence
    (:then_0
      (bind _chargeamount (Timeline|ChargeTimeline Stop)
        (:Update
          (Variables|Default|SetChargeAmount _chargeamount))))
    (:then_1
      (Timeline|ChargeTimeline SetNewTime))))

(event Custom|DestoryArrow
  (Actor|DestroyActor (Variables|Default|GetArrow)))

(fn ConstructionScript)