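; Bow arrow projectile driven by a state machine (In Bow, In Air, Unonbtained) that switches collision and projectile movement.
; Fire stores bow charge and launches it along the Player camera's forward vector, with speed interpolated by charge.
; An in-flight overlap with anything but the player plays a sound, sticks the arrow to that actor and applies damage.
; Once landed, overlap with a Player2 destroys it.
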(event OnComponentBeginOverlap(arrow)
  (params (OverlappedComponent :type Primitive%20Component%20Object%20Reference) (OtherActor :type Actor%20Object%20Reference) (OtherComp :type Primitive%20Component%20Object%20Reference) (OtherBodyIndex :type Integer) (bFromSweep :type Boolean) (SweepResult :type Hit%20Result%20Structure%20%28by%20ref%29))
  (Private|HandleOverlap OtherActor SweepResult))

(event Custom|Fire
  (params (BowCharge :type Float%20%28single-precision%29))
  (Variables|Default|SetBowChargeAmount BowCharge)
  (Private|SetArrowState "NewEnumerator1"))

(fn ConstructionScript)

(fn SetArrowState
  (params (NewState :type E_ArrowState%20Enum :default "NewEnumerator0"))
  (if (!= NewState (Variables|Default|GetArrowState))
    (Private|OnStateEnd "NewEnumerator0")
    (bind _output_get (Variables|Default|SetArrowState NewState))
    (Private|OnStateBegin _output_get)))

(fn OnStateBegin
  (params (State :type E_ArrowState%20Enum :default "NewEnumerator0"))
  (bind _projectilemovement (Variables|Default|GetProjectileMovement))
  ;[1 1 1] New System
  (switch Utilities|FlowControl|Switch|SwitchonE_ArrowState State
    (:NewEnumerator1
      (Collision|SetCollisionProfileName (Variables|Default|Getarrow) "OverlapAllDynamic" true :!class /Script/Engine.PrimitiveComponent)
      (Components|Activation|Activate (Variables|Default|GetProjectileMovement) true)
      (Variables|/Script/Engine.MovementComponent|SetVelocity _projectilemovement (* (Math|Vector|GetForwardVector (Variables|/Game/ThirdPersonBP/Blueprints/Player.Player_C|GetFirstPersonCamera (.AsPlayer (Utilities|Casting|CastToPlayer (Game|GetPlayerCharacter 0))))) (Math|Float|Lerp 2e+03 6e+03 (Variables|Default|GetBowChargeAmount))))
      (Variables|/Script/Engine.ProjectileMovementComponent|SetbRotationFollowsVelocity _projectilemovement true)
      (Variables|/Script/Engine.SkeletalMeshComponent|SetbPauseAnims (Variables|Default|Getcube_) false))
    (:NewEnumerator2
      (Collision|SetCollisionProfileName (Variables|Default|Getarrow) "OverlapAllDynamic" true :!class /Script/Engine.PrimitiveComponent))
    (:NewEnumerator3
      (Collision|SetCollisionProfileName (Variables|Default|Getarrow) "NoCollision" true :!class /Script/Engine.PrimitiveComponent))))

(fn OnStateEnd
  (params (State :type E_ArrowState%20Enum :default "NewEnumerator0"))
  (switch Utilities|FlowControl|Switch|SwitchonE_ArrowState State
    (:NewEnumerator1
      (Components|Activation|Deactivate (Variables|Default|GetProjectileMovement)))))

(fn HandleOverlap
  (params (OtherActor :type Actor%20Object%20Reference) (HitResult :type Hit%20Result%20Structure))
  (switch Utilities|FlowControl|Switch|SwitchonE_ArrowState (Variables|Default|GetArrowState)
    (:NewEnumerator1
      (if (!= OtherActor (Game|GetPlayerCharacter 0))
        (Private|SetArrowState "NewEnumerator2")
        (Audio|PlaySound2D "/Game/weapons/SoundEffects/Bow_Arrow_Sound_Effects_All_Sounds-_AudioTrimmer_com_-_AudioTrimmer_com_.Bow_Arrow_Sound_Effects_All_Sounds-_AudioTrimmer_com_-_AudioTrimmer_com_" 1.0 1.0 0.15 0 0)
        (Components|Activation|Deactivate (Variables|Default|GetProjectileMovement))
        (Transformation|SetActorLocation (- (.impactpoint HitResult) (* (Transformation|GetActorForwardVector) 80)) false true)
        (Transformation|AttachActorToActor OtherActor "None" "KeepWorld" "KeepWorld" "KeepWorld" true)
        (Game|Damage|ApplyDamage (.hitactor HitResult) 5e+01 0 0)))
    (:NewEnumerator2
      (Utilities|Casting|CastToPlayer2 OtherActor)
      (Actor|DestroyActor))))