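; Bow arrow projectile that Player2 fires from the first-person camera, with launch speed scaled by bow charge.
; A state machine (In Bow, In Air, Unonbtained) sets collision and starts projectile movement, with rotation following velocity.
; An in-air overlap with anything but the player stops and attaches the arrow, plays a sound and damages RobotMan.
; A stuck arrow is destroyed when Player2 overlaps it; older line-trace aiming remains unused.
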(event OnComponentBeginOverlap(arrow)
  (params (OverlappedComponent :type Primitive%20Component%20Object%20Reference) (OtherActor :type Actor%20Object%20Reference) (OtherComp :type Primitive%20Component%20Object%20Reference) (OtherBodyIndex :type Integer) (bFromSweep :type Boolean) (SweepResult :type Hit%20Result%20Structure%20%28by%20ref%29))
  (Private|HandleOverlap OtherActor SweepResult))

(event Custom|Fire
  (params (BowCharge :type Float%20%28single-precision%29))
  (Variables|Default|SetBowChargeAmount BowCharge)
  (Private|SetArrowState "NewEnumerator1"))

(fn ConstructionScript)

(fn SetArrowState
  (params (NewState :type E_ArrowState%20Enum :default "NewEnumerator0"))
  (if (!= NewState (Variables|Default|GetArrowState))
    (Private|OnStateEnd "NewEnumerator0")
    (bind _output_get (Variables|Default|SetArrowState NewState))
    (Private|OnStateBegin _output_get)))

(fn OnStateBegin
  (params (State :type E_ArrowState%20Enum :default "NewEnumerator0"))
  (bind _returnvalue (Game|GetPlayerCharacter 0))
  (bind _asplayer_2 (Utilities|Casting|CastToPlayer2 _returnvalue))
  (bind _firstpersoncamera (Variables|/Game/ThirdPersonBP/Blueprints/Player2.Player2_C|GetFirstPersonCamera _asplayer_2))
  (bind _returnvalue_2 (Transformation|GetWorldTransform _firstpersoncamera))
  ;[1 1 1] New System
  (switch Utilities|FlowControl|Switch|SwitchonE_ArrowState State
    (:NewEnumerator1
      (Collision|SetCollisionProfileName (Variables|Default|Getarrow) "OverlapAllDynamic" true :!class /Script/Engine.PrimitiveComponent)
      (Components|Activation|Activate (Variables|Default|GetProjectileMovement) true)
      (Transformation|SetActorTransform (Math|Transform|MakeTransform (.location _returnvalue_2) (.rotation _returnvalue_2) "0.200000,0.400000,0.400000") false true)
      (Variables|/Script/Engine.MovementComponent|SetVelocity (Variables|Default|GetProjectileMovement) (* (Math|Vector|GetForwardVector _firstpersoncamera) (Math|Float|Lerp 2e+03 6e+03 (Variables|Default|GetBowChargeAmount))))
      (Variables|/Script/Engine.ProjectileMovementComponent|SetbRotationFollowsVelocity (Variables|Default|GetProjectileMovement) true))
    (:NewEnumerator2
      (Collision|SetCollisionProfileName (Variables|Default|Getarrow) "OverlapAllDynamic" true :!class /Script/Engine.PrimitiveComponent))
    (:NewEnumerator3
      (Collision|SetCollisionProfileName (Variables|Default|Getarrow) "NoCollision" true :!class /Script/Engine.PrimitiveComponent))))

(fn OnStateEnd
  (params (State :type E_ArrowState%20Enum :default "NewEnumerator0"))
  (switch Utilities|FlowControl|Switch|SwitchonE_ArrowState State
    (:NewEnumerator1
      (Components|Activation|Deactivate (Variables|Default|GetProjectileMovement)))))

(fn HandleOverlap
  (params (OtherActor :type Actor%20Object%20Reference) (HitResult :type Hit%20Result%20Structure))
  (switch Utilities|FlowControl|Switch|SwitchonE_ArrowState (Variables|Default|GetArrowState)
    (:NewEnumerator1
      (if (!= OtherActor (Game|GetPlayerCharacter 0))
        (Private|SetArrowState "NewEnumerator2")
        (Audio|PlaySound2D "/Game/weapons/SoundEffects/Bow_Arrow_Sound_Effects_All_Sounds-_AudioTrimmer_com_-_AudioTrimmer_com_.Bow_Arrow_Sound_Effects_All_Sounds-_AudioTrimmer_com_-_AudioTrimmer_com_" 1.0 1.0 0.15 0 0)
        (Components|Activation|Deactivate (Variables|Default|GetProjectileMovement))
        (Transformation|SetActorLocation (- (.impactpoint HitResult) (* (Transformation|GetActorForwardVector) 80)) false true)
        (Transformation|AttachActorToActor OtherActor "None" "KeepWorld" "KeepWorld" "KeepWorld" true)
        (bind _asrobot_man (Utilities|Casting|CastToRobotMan (.hitactor HitResult)))
        (Variables|/Game/ThirdPersonBP/Blueprints/NPC/NPCBluePrint/RobotMan.RobotMan_C|SetHealth _asrobot_man (- (Variables|/Game/ThirdPersonBP/Blueprints/NPC/NPCBluePrint/RobotMan.RobotMan_C|GetHealth _asrobot_man) 5e+01))
        (Default|CheckHealth _asrobot_man)))
    (:NewEnumerator2
      (Utilities|Casting|CastToPlayer2 OtherActor)
      (Actor|DestroyActor))))