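; Bow weapon Blueprint that handles charging, firing and reloading of BP_Arrow projectiles.
; A timeline drives ChargeAmount, playing forward to charge and reversing on release, with a separate event to stop and reset it.
; Reloading attaches a new arrow at ArrowSocket.
; Firing swaps that arrow for one spawned at Player2's first-person camera with a yaw offset, launches it with ChargeAmount, then clears the reference.
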(event Custom|BeginCharge
  (Variables|Default|GetArrow
    (:then
      (bind _chargeamount (Timeline|ChargeTimeline Play)
        (:Update
          (Variables|Default|SetChargeAmount _chargeamount))))
    (:else)))

(event Custom|ReloadBow
  (bind _returnvalue (Game|SpawnActorfromClass "/Game/weapons/Models/Bow/OldBow/Arrow/BP_Arrow.BP_Arrow_C" (Math|Transform|MakeTransform "0, 0, 0" "0,90.000000, 0" "0.200000,0.400000,0.400000") "AlwaysSpawn" 0 "NewEnumerator3" 0))
  (bind _output_get (Variables|Default|SetArrow _returnvalue))
  (Transformation|AttachComponentToComponent _output_get (Variables|Default|Getall) "ArrowSocket" "KeepRelative" "KeepRelative" "KeepWorld" true))

(event Custom|EndCharge
  (Variables|Default|GetArrow
    (:then
      (bind _chargeamount (Timeline|ChargeTimeline Reverse)
        (:Update
          (Variables|Default|SetChargeAmount _chargeamount))))
    (:else)))

(event Custom|Fire
  (bind _returnvalue (Game|GetPlayerCharacter 0))
  (bind _asplayer_2 (Utilities|Casting|CastToPlayer2 _returnvalue))
  (bind _firstpersoncamera (Variables|/Game/ThirdPersonBP/Blueprints/Player2.Player2_C|GetFirstPersonCamera _asplayer_2))
  (bind _returnvalue_2 (Transformation|GetWorldTransform _firstpersoncamera))
  (Variables|Default|GetArrow
    (:then
      (Actor|DestroyActor (Variables|Default|GetArrow))
      (bind _returnvalue_3 (Game|SpawnActorfromClass "/Game/weapons/Models/Bow/OldBow/Arrow/BP_Arrow.BP_Arrow_C" (Math|Transform|MakeTransform (.location _returnvalue_2) (Math|Rotator|MakeRotator (.roll (.rotation _returnvalue_2)) (.pitch (.rotation _returnvalue_2)) (+ (.yaw (.rotation _returnvalue_2)) 9e+01)) "0.200000,0.400000,0.400000") "AlwaysSpawn" 0 "NewEnumerator3" 0))
      (bind _output_get (Variables|Default|SetArrow _returnvalue_3))
      (Default|Fire _output_get (Variables|Default|GetChargeAmount))
      (Variables|Default|SetArrow 0))
    (:else)))

(event Custom|StopCharge
  (Utilities|FlowControl|Sequence
    (:then_0
      (bind _chargeamount (Timeline|ChargeTimeline Stop)
        (:Update
          (Variables|Default|SetChargeAmount _chargeamount))))
    (:then_1
      (Timeline|ChargeTimeline SetNewTime))))

(event Custom|DestoryArrow
  (Actor|DestroyActor (Variables|Default|GetArrow)))

(fn ConstructionScript)