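; Shooting target prop that drops when hit, pops back up after a random delay, and can be destroyed by explosion.
; Tick polls hit and explode flags, which this graph never triggers itself, with guard booleans preventing repeat sounds and explosions.
; Hits play down and up animations with sounds while toggling the active state.
; Exploding spawns a destroyed-target actor, fires a radial impulse randomized at BeginPlay, then destroys itself.
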(event EventTick
  (params (DeltaSeconds :type Float%20%28single-precision%29))
  (bind _target_animated (Variables|Default|Gettarget_animated))
  (bind _target_animated_2 (Variables|Default|Gettarget_animated))
  (bind _returnvalue (Transformation|GetWorldLocation _target_animated))
  (Utilities|FlowControl|Sequence
    (:then_0
      (if (and (Variables|Default|GettargetHasBeenHit) (not (Variables|Default|GettargetHasExploded))) ; Check if target has been hit
        (Utilities|FlowControl|Sequence
          (:then_0
            (Variables|Default|SetisActive false)
            (if (not (Variables|Default|GetsoundHasPlayed)) ; If sound has not played yet
              (Audio|PlaySoundatLocation "/Game/Low_Poly_FPS_Pack/Content/Audio/WAV/Misc/S_target_go_down.S_target_go_down" _returnvalue) ; Play sound effect at target location
              (Variables|Default|SetsoundHasPlayed true)
              (Components|Animation|PlayAnimation (Variables|Default|Gettarget_animated) "/Game/Low_Poly_FPS_Pack/Content/Animations/Sequences/Demo_Maps/Target/target_down_Anim.target_down_Anim" false) ; Play target down animation
            ))
          (:then_1
            (Utilities|FlowControl|Delay (Math|Random|RandomFloatinRange (Variables|Default|GetminTargetDelay) (Variables|Default|GetmaxTargetDelay))) ; Wait for random amount of time
            (Variables|Default|SettargetHasBeenHit false)
            (Variables|Default|SetisActive true) ; Activate target again
            (Audio|PlaySoundatLocation "/Game/Low_Poly_FPS_Pack/Content/Audio/WAV/Misc/S_target_go_up.S_target_go_up" _returnvalue "0, 0, 0" 1.0 1.0 0.0 "/Game/Low_Poly_FPS_Pack/Content/Audio/Sound_Attenuation/SoundAttenuation_Main.SoundAttenuation_Main")
            (Variables|Default|SetsoundHasPlayed false)
            (Components|Animation|PlayAnimation (Variables|Default|Gettarget_animated) "/Game/Low_Poly_FPS_Pack/Content/Animations/Sequences/Demo_Maps/Target/target_up_Anim.target_up_Anim" false) ; Play target up animation
          ))))
    (:then_1
      (if (and (Variables|Default|GetexplodeTarget) (not (Variables|Default|GettargetHasExploded)))
        (Variables|Default|SetexplodeTarget false)
        (Variables|Default|SettargetHasExploded true)
        (Game|SpawnActorfromClass "/Game/Low_Poly_FPS_Pack/Content/Blueprints/Demo_Maps/Enivronment_Props/Target/Destroyed/BP_Target_Destroyed.BP_Target_Destroyed_C" (Math|Transform|MakeTransform (Transformation|GetWorldLocation _target_animated_2) (Transformation|GetWorldRotation _target_animated_2) "1,1,1") "AlwaysSpawn" 0 0) ; Spawn destroyed target
        (Class|RadialForceComponent|FireImpulse (Variables|Default|GetRadialForce))
        (Actor|DestroyActor) ; Destroy target actor
      ))))

(event EventBeginPlay
  (bind _returnvalue (Math|Random|RandomFloatinRange 5e+02 2.5e+03))
  (bind _radialforce (Variables|Default|GetRadialForce))
  (Variables|/Script/Engine.RadialForceComponent|SetImpulseStrength _radialforce _returnvalue)
  (Variables|/Script/Engine.RadialForceComponent|SetForceStrength _radialforce _returnvalue)
  (Variables|/Script/Engine.RadialForceComponent|SetRadius _radialforce (Math|Random|RandomFloatinRange 5e+01 1.5e+02)))

(fn ConstructionScript)