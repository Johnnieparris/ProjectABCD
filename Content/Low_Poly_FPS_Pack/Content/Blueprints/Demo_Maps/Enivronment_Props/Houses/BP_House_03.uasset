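; Destructible house prop that blows apart once when its Explode flag is set, which Tick polls.
; ExplodeHouse swaps the house, door and window hatches for a destroyed house and physics actors, then fires a radial impulse and spawns explosion and fire particles.
; SpawnDecal follows shortly, line tracing to the ground to add randomly sized effects and a burn decal, before the actor destroys itself.
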(event EventTick
  (params (DeltaSeconds :type Float%20%28single-precision%29))
  (if (and (Variables|Default|Getexplode) (not (Variables|Default|GethouseHasExploded)))
    (Variables|Default|Setexplode false)
    (Variables|Default|SethouseHasExploded true)
    (CallFunction|ExplodeHouse)
    (Utilities|FlowControl|Delay 0.15)
    (CallFunction|SpawnDecal)
    (Utilities|FlowControl|Delay 1.0)
    (Actor|DestroyActor)))

(fn ConstructionScript)

(fn ExplodeHouse
  (bind _door_spawn_point (Variables|Default|GetDoor_Spawn_Point))
  (bind _door_explosion_spawn_point (Variables|Default|GetDoor_Explosion_Spawn_Point))
  (bind _house_mesh (Variables|Default|GetHouse_Mesh))
  (Utilities|FlowControl|Sequence
    (:then_0
      (Components|DestroyComponent (Variables|Default|GetBP_House_Door)) ; Destroy current door mesh
      (Game|SpawnActorfromClass "/Game/Low_Poly_FPS_Pack/Content/Blueprints/Demo_Maps/Enivronment_Props/Houses/Doors_Windows/BP_House_Door_Physics.BP_House_Door_Physics_C" (Math|Transform|MakeTransform (Transformation|GetWorldLocation _door_spawn_point) (Transformation|GetWorldRotation _door_spawn_point) "1,1,1") "Undefined" 0 0) ; Spawn physics door mesh at spawn point
      (Collision|SetCollisionEnabled _house_mesh "NoCollision") ; Disable collision for current house mesh
      (Game|SpawnActorfromClass "/Game/Low_Poly_FPS_Pack/Content/Blueprints/Demo_Maps/Enivronment_Props/Houses/House_03_Destroyed/BP_House_03_Destroyed.BP_House_03_Destroyed_C" (Math|Transform|MakeTransform (Transformation|GetWorldLocation _house_mesh) (Transformation|GetWorldRotation _house_mesh) (Transformation|GetWorldScale _house_mesh)) "AdjustIfPossibleButAlwaysSpawn" 0 0) ; Spawn destroyed house
      (Rendering|SetVisibility _house_mesh false false) ; Hide/disable visibility for current house mesh
      (Class|RadialForceComponent|FireImpulse (Variables|Default|GetRadialForce)) ; Fire  impulse after spawning destroyed house
    )
    (:then_1
      (Effects|SpawnEmitteratLocation "/Game/Low_Poly_FPS_Pack/Content/Particle_Systems/Explosions/PS_Door_Explosion.PS_Door_Explosion" (Transformation|GetWorldLocation _door_explosion_spawn_point) (Transformation|GetWorldRotation _door_explosion_spawn_point)) ; Spawn explosion particles
      (Effects|SpawnEmitteratLocation "/Game/Low_Poly_FPS_Pack/Content/Particle_Systems/Flames/PS_Flames_House.PS_Flames_House" (Transformation|GetWorldLocation (Variables|Default|GetHouse_Mesh))) ; Spawn flames and smoke particles
    )
    (:then_2
      (for _array_element (Utilities|Array|MakeArray (Variables|Default|GetWindow_Hatch_01) (Variables|Default|GetWindow_Hatch_02) (Variables|Default|GetWindow_Hatch_03) (Variables|Default|GetWindow_Hatch_04) (Variables|Default|GetWindow_Hatch_05) (Variables|Default|GetWindow_Hatch_06) (Variables|Default|GetWindow_Hatch_07) (Variables|Default|GetWindow_Hatch_08))
        (Game|SpawnActorfromClass "/Game/Low_Poly_FPS_Pack/Content/Blueprints/Demo_Maps/Enivronment_Props/Houses/Doors_Windows/BP_House_Window_Physics.BP_House_Window_Physics_C" (Math|Transform|MakeTransform (Transformation|GetWorldLocation _array_element) (Transformation|GetWorldRotation _array_element) "1,1,1") "AdjustIfPossibleButAlwaysSpawn" 0 0) ; Spawn physics based window hatches at same locations
        (Components|DestroyComponent _array_element) ; Destroy current window hatch meshes
      ))))

(fn SpawnDecal
  (bind _returnvalue (Math|Random|RandomFloatinRange 1.4e+03 1.7e+03))
  (bind _trace_ground_check (Variables|Default|GetTrace_Ground_Check))
  (bind _returnvalue_2 (Transformation|GetWorldLocation _trace_ground_check))
  ;[1 1 1] Spawn Explosion Particles
  (bind (_outhit _returnvalue_3) (Collision|LineTraceByChannel _returnvalue_2 (+ _returnvalue_2 (* (Math|Vector|GetForwardVector _trace_ground_check) 2.5e+04)) "TraceTypeQuery1" false 0 "None")) ; Check where the ground is on explosion
  (if _returnvalue_3
    (Utilities|FlowControl|Sequence
      (:then_0
        (Effects|SpawnEmitteratLocation "/Game/Low_Poly_FPS_Pack/Content/Particle_Systems/Explosions/PS_Explosion.PS_Explosion" (.Location (Collision|BreakHitResult _outhit)) "0, 0, 0" (Math|Conversions|ToVector(Float) (Math|Random|RandomFloatinRange 0.8 1.2))) ; Spawn explosion particles
        (Effects|SpawnEmitteratLocation "/Game/Low_Poly_FPS_Pack/Content/Particle_Systems/Flames/PS_Flames_Barrel.PS_Flames_Barrel" (.Location (Collision|BreakHitResult _outhit)) "0, 0, 0" (Math|Conversions|ToVector(Float) (Math|Random|RandomFloatinRange 0.7 2.0))) ; Spawn flames particles
      )
      (:then_1
        (bind _returnvalue_4 (Rendering|Decal|SpawnDecalatLocation "/Game/Low_Poly_FPS_Pack/Content/Materials/Material_Instances/Decals/MI_Decal_Burn_Mark_02.MI_Decal_Burn_Mark_02" (Math|Vector|MakeVector _returnvalue _returnvalue _returnvalue) (.Location (Collision|BreakHitResult _outhit)) (Math|Conversions|RotationFromXVector (.TraceEnd (Collision|BreakHitResult _outhit))) (Variables|Default|GetdecalDestroyTimer))) ; Spawn burn mark decal on line trace hit location
        (Transformation|SetRelativeRotation _returnvalue_4 (Math|Rotator|MakeRotator (Math|Random|RandomFloatinRange 0.0 3.6e+02) (.Pitch (Math|Rotator|BreakRotator (Math|Conversions|RotationFromXVector (.TraceEnd (Collision|BreakHitResult _outhit))))) (.Yaw (Math|Rotator|BreakRotator (Math|Conversions|RotationFromXVector (.TraceEnd (Collision|BreakHitResult _outhit)))))) false false) ; Set random decal rotation
      ))))