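; BP_House_03_Destroyed is a destroyed house prop made of physics debris pieces that removes itself after DestroyTimer seconds.
; Until PhysicsDisabled is set, Tick waits a random short delay, then loops over the seventeen mesh components.
; Pieces whose signed X, Y and Z velocities are all below MinKillVelocity stop simulating physics.
; The first such freeze also starts a delay that sets PhysicsDisabled, ending further checks.
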(event EventBeginPlay
  (Utilities|FlowControl|Delay (Variables|Default|GetdestroyTimer))
  (Actor|DestroyActor) ; Destroy house actor after set amount of time
)

(event EventTick
  (params (DeltaSeconds :type Float%20%28single-precision%29))
  (bind _minkillvelocity (Variables|Default|GetminKillVelocity))
  (if (not (Variables|Default|GetphysicsDisabled)) ; Keep checking if physics are not disabled
    (Utilities|FlowControl|Delay (Math|Random|RandomFloatinRange 2.0 4.0)) ; Check delay
    (for _array_element (Utilities|Array|MakeArray (Variables|Default|GetSM_house_03_destroyed_001) (Variables|Default|GetSM_house_03_destroyed_002) (Variables|Default|GetSM_house_03_destroyed_003) (Variables|Default|GetSM_house_03_destroyed_004) (Variables|Default|GetSM_house_03_destroyed_005) (Variables|Default|GetSM_house_03_destroyed_006) (Variables|Default|GetSM_house_03_destroyed_007) (Variables|Default|GetSM_house_03_destroyed_008) (Variables|Default|GetSM_house_03_destroyed_009) (Variables|Default|GetSM_house_03_destroyed_010) (Variables|Default|GetSM_house_03_destroyed_011) (Variables|Default|GetSM_house_03_destroyed_012) (Variables|Default|GetSM_house_03_destroyed_013) (Variables|Default|GetSM_house_03_destroyed_014) (Variables|Default|GetSM_house_03_destroyed_015) (Variables|Default|GetSM_house_03_destroyed_016) (Variables|Default|GetSM_house_03_destroyed_017)) ; Check all components in array
      (if (Math|Boolean|ANDBoolean (< (.x (Transformation|GetComponentVelocity _array_element)) _minkillvelocity) (< (.y (Transformation|GetComponentVelocity _array_element)) _minkillvelocity) (< (.z (Transformation|GetComponentVelocity _array_element)) _minkillvelocity)) ; Check if components velocity value is less than "minKillVelocity"
        (Physics|SetSimulatePhysics _array_element false) ; Disable physics simlation
        (Utilities|FlowControl|Delay 5.0)
        (Variables|Default|SetphysicsDisabled true) ; Disable check for velocity
      ))))

(fn ConstructionScript)