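; BP_House_Explosion_Area is a helper actor that relays a one-time explode trigger to the house Blueprint that parents it.
; Tick polls the ExplodeHouse flag, which nothing in this graph sets to true, and latches HouseHasExploded so it fires only once.
; It then tries casting its parent actor to BP_House_01, 02 and 03 in sequence, setting Explode on whichever matches.
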(event EventTick
  (params (DeltaSeconds :type Float%20%28single-precision%29))
  (bind _returnvalue (Actor|GetParentActor))
  (if (and (Variables|Default|GetexplodeHouse) (not (Variables|Default|GethouseHasExploded)))
    (Variables|Default|SetexplodeHouse false)
    (Variables|Default|SethouseHasExploded true)
    (Utilities|FlowControl|Sequence
      (:then_0
        (bind _asbp_house_01 (Utilities|Casting|CastToBP_House_01 _returnvalue))
        (Variables|/Game/Low_Poly_FPS_Pack/Content/Blueprints/Demo_Maps/Enivronment_Props/Houses/BP_House_01.BP_House_01_C|Setexplode _asbp_house_01 true))
      (:then_1
        (bind _asbp_house_02 (Utilities|Casting|CastToBP_House_02 _returnvalue))
        (Variables|/Game/Low_Poly_FPS_Pack/Content/Blueprints/Demo_Maps/Enivronment_Props/Houses/BP_House_02.BP_House_02_C|Setexplode _asbp_house_02 true))
      (:then_2
        (bind _asbp_house_03 (Utilities|Casting|CastToBP_House_03 _returnvalue))
        (Variables|/Game/Low_Poly_FPS_Pack/Content/Blueprints/Demo_Maps/Enivronment_Props/Houses/BP_House_03.BP_House_03_C|Setexplode _asbp_house_03 true)))))

(fn ConstructionScript)