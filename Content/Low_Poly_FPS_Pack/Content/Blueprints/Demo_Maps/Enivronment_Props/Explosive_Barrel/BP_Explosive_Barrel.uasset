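; Explosive barrel prop that explodes immediately when hit by a bullet, or after a random delay when flagged as hit by another explosion.
; Randomizes radial force at BeginPlay and polls the hit flag on Tick.
; Explode spawns ground-traced effects and a scorch decal, swaps in a destroyed barrel, fires an impulse, sound and camera shake.
; A sphere overlap flags nearby props and characters for chain reactions and damages RobotMan, before the actor self-destroys.
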(event OnComponentHit(explosive_barrel)
  (params (HitComponent :type Primitive%20Component%20Object%20Reference) (OtherActor :type Actor%20Object%20Reference) (OtherComp :type Primitive%20Component%20Object%20Reference) (NormalImpulse :type Vector :default "0, 0, 0") (Hit :type Hit%20Result%20Structure%20%28by%20ref%29))
  (Utilities|Casting|CastToBulletClass OtherActor)
  ;[0 0.7656 1] Check if explosive barrel is hit
  (CallFunction|Explode)
  (Utilities|FlowControl|Delay 1.5)
  (Actor|DestroyActor) ; Destroy explosive barrel
)

(event EventBeginPlay
  (bind _radialforce (Variables|Default|GetRadialForce))
  (Utilities|FlowControl|Sequence
    (:then_0
      ;[1 0 0.04687] Set Radial Force Radius
      (Variables|/Script/Engine.RadialForceComponent|SetRadius _radialforce (Math|Random|RandomFloatinRange (Variables|ExplosionSettings|GetminExplosionRadius) (Variables|ExplosionSettings|GetmaxExplosionRadius))))
    (:then_1
      ;[0 1 0.8828] Set Radial Force Strength
      (Variables|/Script/Engine.RadialForceComponent|SetForceStrength _radialforce (Math|Random|RandomFloatinRange (Variables|ExplosionSettings|GetminForceStrength) (Variables|ExplosionSettings|GetmaxForceStrength))))
    (:then_2
      ;[0.8516 0 1] Set Radial Force Impulse Strength
      (Variables|/Script/Engine.RadialForceComponent|SetImpulseStrength _radialforce (Math|Random|RandomFloatinRange (Variables|ExplosionSettings|GetminImpulseStrength) (Variables|ExplosionSettings|GetmaxImpulseStrength))))))

(event EventTick
  (params (DeltaSeconds :type Float%20%28single-precision%29))
  ;[0 0.7656 1] Check if explosive barrel is hit
  (if (and (Variables|Default|GetbarrelIsHit) (Variables|Default|GetisInactive)) ; Check if barrel is hit
    (Variables|Default|SetbarrelIsHit false)
    (Variables|Default|SetisInactive false)
    (Utilities|FlowControl|Delay (Math|Random|RandomFloatinRange (Variables|ExplosionSettings|GetminExplodeTimer) (Variables|ExplosionSettings|GetmaxExplodeTimer))) ; Wait for random amount of time before exploding
    (CallFunction|Explode)
    (Utilities|FlowControl|Delay 1.5)
    (Actor|DestroyActor) ; Destroy explosive barrel
  ))

(fn ConstructionScript)

(fn Explode
  (bind _returnvalue (Math|Random|RandomFloatinRange 1e+02 3e+02))
  (bind _radialforce (Variables|Default|GetRadialForce))
  (bind _explosive_barrel (Variables|Default|Getexplosive_barrel))
  ;[0 1 0.4375] Explode
  (Utilities|FlowControl|Sequence
    (:then_0
      ;[1 0.2812 0] Spawn Explosion Particles
      (bind (_outhit _returnvalue_2) (Collision|LineTraceByChannel (Transformation|GetWorldLocation (Variables|Default|Getexplosive_barrel)) "0, 0,-5000.000000" "TraceTypeQuery1" false 0 "None")) ; Check where the ground is on explosion
      (if _returnvalue_2
        (Utilities|FlowControl|Sequence
          (:then_0
            (Effects|SpawnEmitteratLocation "/Game/Low_Poly_FPS_Pack/Content/Particle_Systems/Explosions/PS_Explosion.PS_Explosion" (.Location (Collision|BreakHitResult _outhit)) "0, 0, 0" (Math|Conversions|ToVector(Float) (Math|Random|RandomFloatinRange 0.8 1.2))) ; Spawn explosion particles
            (Effects|SpawnEmitteratLocation "/Game/Low_Poly_FPS_Pack/Content/Particle_Systems/Flames/PS_Flames_Barrel.PS_Flames_Barrel" (.Location (Collision|BreakHitResult _outhit)) "0, 0, 0" (Math|Conversions|ToVector(Float) (Math|Random|RandomFloatinRange 0.7 2.0))) ; Spawn flames particles
            (Game|SpawnActorfromClass "/Game/Low_Poly_FPS_Pack/Content/Blueprints/Demo_Maps/Effects/BP_Heat_Distortion_Effect.BP_Heat_Distortion_Effect_C" (Math|Transform|MakeTransform (.Location (Collision|BreakHitResult _outhit)) "0, 0, 0" "1,1,1") "AlwaysSpawn" 0 0) ; Spawn heat distortion effect
            (Game|SpawnActorfromClass "/Game/Low_Poly_FPS_Pack/Content/Blueprints/Demo_Maps/Effects/BP_Flame_Light_Effect.BP_Flame_Light_Effect_C" (Math|Transform|MakeTransform (.Location (Collision|BreakHitResult _outhit)) "0, 0, 0" "1,1,1") "AlwaysSpawn" 0 0) ; Spawn flame light effect
          )
          (:then_1
            (bind _returnvalue_3 (Rendering|Decal|SpawnDecalatLocation "/Game/Low_Poly_FPS_Pack/Content/Materials/Base_Materials/M_Decal_Base.M_Decal_Base" (Math|Vector|MakeVector _returnvalue _returnvalue _returnvalue) (.Location (Collision|BreakHitResult _outhit)) (Math|Conversions|RotationFromXVector (.Normal (Collision|BreakHitResult _outhit))) (Variables|Default|GetdecalDestroyTimer))) ; Spawn burn mark decal on line trace hit location
            (Transformation|SetRelativeRotation _returnvalue_3 (Math|Rotator|MakeRotator (Math|Random|RandomFloatinRange 0.0 3.6e+02) (.Pitch (Math|Rotator|BreakRotator (Math|Conversions|RotationFromXVector (.Normal (Collision|BreakHitResult _outhit))))) (.Yaw (Math|Rotator|BreakRotator (Math|Conversions|RotationFromXVector (.Normal (Collision|BreakHitResult _outhit)))))) false false) ; Set random decal rotation
          ))))
    (:then_1
      (Game|SpawnActorfromClass "/Game/Low_Poly_FPS_Pack/Content/Blueprints/Demo_Maps/Enivronment_Props/Explosive_Barrel/Destroyed/BP_Destroyed_Barrel.BP_Destroyed_Barrel_C" (Transformation|GetWorldTransform _radialforce) "AlwaysSpawn" 0 0) ; Spawn destroyed barrel
      (Class|RadialForceComponent|FireImpulse (Variables|Default|GetRadialForce)) ; Fire radial force impulse
      (Rendering|SetVisibility _explosive_barrel false false) ; Hide the current barrel actor
      (Physics|SetSimulatePhysics _explosive_barrel false) ; Freeze barrel physics
      (Collision|SetCollisionEnabled _explosive_barrel "NoCollision") ; Disable collision for current barrel actor
      (Camera|PlayWorldCameraShake "/Game/Low_Poly_FPS_Pack/Content/Blueprints/Camera_Shake/BP_Camera_Shake_Big.BP_Camera_Shake_Big_C" (Transformation|GetWorldLocation (Variables|Default|Getexplosive_barrel)) 0.0 5e+03 1.0 true))
    (:then_2
      (bind (_outactors _returnvalue_4) (Collision|SphereOverlapActors (Transformation|GetWorldLocation _radialforce) (Math|Random|RandomFloatinRange (Variables|ExplosionSettings|GetminExplosionRadius) (Variables|ExplosionSettings|GetmaxExplosionRadius)) (Utilities|Array|MakeArray "ObjectTypeQuery4" "ObjectTypeQuery2" "ObjectTypeQuery1" "ObjectTypeQuery3") 0)) ; Check actors within random sphere radius
      (if _returnvalue_4
        (for _array_element _outactors ; Check all actors hit by sphere overlap
          (Utilities|FlowControl|Sequence
            (:then_0
              ;[0.03125 0 1] Check which actors got hit by sphere overlap
              (bind _asbp_target (Utilities|Casting|CastToBP_Target _array_element)) ; If explosion hits target
              (if (not (Variables|/Game/Low_Poly_FPS_Pack/Content/Blueprints/Demo_Maps/Enivronment_Props/Target/BP_Target.BP_Target_C|GettargetHasExploded _asbp_target))
                (Variables|/Game/Low_Poly_FPS_Pack/Content/Blueprints/Demo_Maps/Enivronment_Props/Target/BP_Target.BP_Target_C|SetexplodeTarget _asbp_target true)))
            (:then_1
              (bind _asbp_explosive_barrel (Utilities|Casting|CastToBP_Explosive_Barrel _array_element)) ; If explosion hits other explosive barrels
              (if (not (Variables|BP_Explosive_Barrel_C|GetbarrelIsHit _asbp_explosive_barrel))
                (Variables|BP_Explosive_Barrel_C|SetbarrelIsHit _asbp_explosive_barrel true)))
            (:then_2
              (bind _asbp_gas_tank (Utilities|Casting|CastToBP_Gas_Tank _array_element)) ; If explosion hits other gas tanks
              (if (not (Variables|/Game/Low_Poly_FPS_Pack/Content/Blueprints/Demo_Maps/Enivronment_Props/Gas_Tank/BP_Gas_Tank.BP_Gas_Tank_C|GetgasTankIsHit _asbp_gas_tank))
                (Variables|/Game/Low_Poly_FPS_Pack/Content/Blueprints/Demo_Maps/Enivronment_Props/Gas_Tank/BP_Gas_Tank.BP_Gas_Tank_C|SetgasTankIsHit _asbp_gas_tank true)))
            (:then_3
              (bind _asbp_stone_wall (Utilities|Casting|CastToBP_Stone_Wall _array_element)) ; If explosion hits stone wall
              (if (not (Variables|/Game/Low_Poly_FPS_Pack/Content/Blueprints/Demo_Maps/Enivronment_Props/Stone_Wall/BP_Stone_Wall.BP_Stone_Wall_C|GetwallHasExploded _asbp_stone_wall))
                (Variables|/Game/Low_Poly_FPS_Pack/Content/Blueprints/Demo_Maps/Enivronment_Props/Stone_Wall/BP_Stone_Wall.BP_Stone_Wall_C|SetexplodeWall _asbp_stone_wall true)))
            (:then_4
              (bind _asbp_house_explosion_area (Utilities|Casting|CastToBP_House_Explosion_Area _array_element)) ; If explosion hits any house
              (if (not (Variables|/Game/Low_Poly_FPS_Pack/Content/Blueprints/Demo_Maps/Enivronment_Props/Houses/Explosion_Area/BP_House_Explosion_Area.BP_House_Explosion_Area_C|GethouseHasExploded _asbp_house_explosion_area))
                (Variables|/Game/Low_Poly_FPS_Pack/Content/Blueprints/Demo_Maps/Enivronment_Props/Houses/Explosion_Area/BP_House_Explosion_Area.BP_House_Explosion_Area_C|SetexplodeHouse _asbp_house_explosion_area true)))
            (:then_5
              (bind _asbp_watchtower (Utilities|Casting|CastToBP_Watchtower _array_element)) ; If explosion hits watchtower
              (if (not (Variables|/Game/Low_Poly_FPS_Pack/Content/Blueprints/Demo_Maps/Enivronment_Props/Watchtower/BP_Watchtower.BP_Watchtower_C|GethasExploded _asbp_watchtower))
                (Variables|/Game/Low_Poly_FPS_Pack/Content/Blueprints/Demo_Maps/Enivronment_Props/Watchtower/BP_Watchtower.BP_Watchtower_C|Setexplode _asbp_watchtower true)))
            (:then_6
              (bind _asbp_tpc_weapon_base (Utilities|Casting|CastToBP_TPC_Weapon_Base _array_element)) ; If explosion hits third person character
              (if (not (Variables|/Game/Low_Poly_FPS_Pack/Content/Blueprints/Third_Person_Character/Base/BP_TPC_Weapon_Base.BP_TPC_Weapon_Base_C|GethasRagdolled _asbp_tpc_weapon_base))
                (Variables|/Game/Low_Poly_FPS_Pack/Content/Blueprints/Third_Person_Character/Base/BP_TPC_Weapon_Base.BP_TPC_Weapon_Base_C|SetenableRagdoll _asbp_tpc_weapon_base true)))
            (:then_7
              (bind _asrobot_man (Utilities|Casting|CastToRobotMan _array_element))
              (Default|TakeDamage _asrobot_man "None" 1e+02))))))
    (:then_3
      ;[1 0 0.4453] Play explosion sound effect
      (Audio|PlaySoundatLocation "/Game/Low_Poly_FPS_Pack/Content/Audio/Sound_Cues/Explosions/SC_Explosion_Random.SC_Explosion_Random" (Transformation|GetWorldLocation (Variables|Default|Getexplosive_barrel)) "0, 0, 0" 1.0 1.0 0.0 "/Game/Low_Poly_FPS_Pack/Content/Audio/Sound_Attenuation/SoundAttenuation_Main.SoundAttenuation_Main" 0 0))))